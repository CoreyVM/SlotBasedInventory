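; ItemBox is a pickup prop that signals when the player is close enough to interact with it.
; Its BoxCollision overlap events cast to ThirdPersonCharacter and set that character's InRangeOfItem flag on enter and exit.
; A Cylinder mesh, hidden at BeginPlay, serves as a prompt, shown with the PickUpIcon_Mat material while the character is in range.
; The pickup action itself is not handled here.
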(event OnComponentBeginOverlap(BoxCollision)
  (params (OverlappedComponent :type Primitive%20Component%20Object%20Reference) (OtherActor :type Actor%20Object%20Reference) (OtherComp :type Primitive%20Component%20Object%20Reference) (OtherBodyIndex :type Integer) (bFromSweep :type Boolean) (SweepResult :type Hit%20Result%20Structure%20%28by%20ref%29))
  (bind _cylinder (Variables|Default|GetCylinder))
  (bind _asthird_person_character (Utilities|Casting|CastToThirdPersonCharacter OtherActor))
  (Variables|/Script/TPSH.TPSHCharacter|SetInRangeOfItem _asthird_person_character true)
  (Rendering|SetVisibility _cylinder true false)
  (Rendering|Material|SetMaterial _cylinder 0 "/Game/Widgets/Icons/PickUpIcon_Mat.PickUpIcon_Mat"))

(event OnComponentEndOverlap(BoxCollision)
  (params (OverlappedComponent :type Primitive%20Component%20Object%20Reference) (OtherActor :type Actor%20Object%20Reference) (OtherComp :type Primitive%20Component%20Object%20Reference) (OtherBodyIndex :type Integer))
  (bind _asthird_person_character (Utilities|Casting|CastToThirdPersonCharacter OtherActor))
  (Variables|/Script/TPSH.TPSHCharacter|SetInRangeOfItem _asthird_person_character false)
  (Rendering|SetVisibility (Variables|Default|GetCylinder) false false))

(event EventBeginPlay
  (Rendering|SetVisibility (Variables|Default|GetCylinder) false false))

(event Collision|EventActorBeginOverlap
  (params (OtherActor :type Actor%20Object%20Reference)))

(event EventTick
  (params (DeltaSeconds :type Float%20%28single-precision%29)))

(fn ConstructionScript)